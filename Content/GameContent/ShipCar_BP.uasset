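; ShipCar_BP is a player-controlled pawn with axis-driven movement and a spring arm.
; Vertical and horizontal move axes feed movement input along the actor's forward and right vectors, while mouse axes add controller yaw and pitch.
; The scroll axis adjusts the spring arm length without clamping, and releasing the left mouse button prints a debug greeting.
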(event EventBeginPlay)

(event Input|ActionEvents|InputActionMouseLeft
  (params (Key :type Key%20Structure :default "None"))
  (:Released
    (Development|PrintString "Hola Unreal!" true true "(R=0.000000,G=1.000000,B=0.324658,A=1.000000)")))

(event Input|AxisEvents|InputAxisHorizontalMouse
  (params (AxisValue :type Float%20%28single-precision%29))
  (Pawn|Input|AddControllerYawInput AxisValue))

(event Input|AxisEvents|InputAxisVerticalMouse
  (params (AxisValue :type Float%20%28single-precision%29))
  (Pawn|Input|AddControllerPitchInput AxisValue))

(event Input|AxisEvents|InputAxisScrollMouse
  (params (AxisValue :type Float%20%28single-precision%29))
  (Variables|/Script/Engine.SpringArmComponent|SetTargetArmLength (Variables|Default|GetSpringArm) (+ (* AxisValue 1e+01) (Variables|/Script/Engine.SpringArmComponent|GetTargetArmLength (Variables|Default|GetSpringArm)))))

(event Input|AxisEvents|InputAxisMoveVertical
  (params (AxisValue :type Float%20%28single-precision%29))
  ;[1 1 1] Movement
  (Pawn|Input|AddMovementInput (Transformation|GetActorForwardVector) AxisValue false))

(event Input|AxisEvents|InputAxisMoveHorizontal
  (params (AxisValue :type Float%20%28single-precision%29))
  ;[1 1 1] Movement
  (Pawn|Input|AddMovementInput (Transformation|GetActorRightVector) AxisValue false))

(fn ConstructionScript)